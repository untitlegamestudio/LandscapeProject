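; BP_PCG_Fence is a fence actor whose construction script derives parameters, presumably for PCG spline fence placement as its name and folder suggest.
; It stores the soft object path of the chosen mesh in MeshPath.
; It splits RandomRotation into a range centered on zero, with RotationMin as the positive half and RotationMax as its negation, despite their names.
; The event graph has no active logic.
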(event EventBeginPlay)

(event Collision|EventActorBeginOverlap
  (params (OtherActor :type Actor%20Object%20Reference)))

(event EventTick
  (params (DeltaSeconds :type Float%20%28single-precision%29)))

(fn ConstructionScript
  (bind _randomrotation (Variables|Default|GetRandomRotation))
  (bind _returnvalue (/ (.yaw _randomrotation) 2.0))
  (bind _returnvalue_2 (/ (.roll _randomrotation) 2.0))
  (bind _returnvalue_3 (/ (.pitch _randomrotation) 2.0))
  (bind _returnvalue_4 (Math|Rotator|MakeRotator _returnvalue_2 _returnvalue_3 _returnvalue))
  (Variables|Default|SetMeshPath (Utilities|GetSoftObjectPath (Variables|Default|GetMesh)))
  (Variables|Default|SetRotationMin _returnvalue_4)
  (Variables|Default|SetRotationMax (* _returnvalue_4 -1.0)))